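; Functional test for maze completion, judging by its name, that checks whether the player character is near a target point.
; Every Tick, it gets a TargetPoint actor in the level and measures its distance to the player character.
; Within a large fixed radius it calls FinishTest with a Default result; otherwise it only prints a debug string.
; PrepareTest, StartTest and BeginPlay hold no logic.
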(event EventPrepareTest)

(event EventStartTest)

(event EventBeginPlay)

(event EventTick
  (params (DeltaSeconds :type Float%20%28single-precision%29))
  (bind _returnvalue (Actor|GetActorOfClass "/Script/Engine.TargetPoint"))
  (Development|PrintString "Hello")
  (if (< (Math|Float|Absolute(Float) (Math|Vector|Distance(Vector) (Transformation|GetActorLocation _returnvalue) (Transformation|GetActorLocation (Game|GetPlayerCharacter 0)))) 1e+04)
    (Development|PrintString "Yesss Hello")
    (Class|FunctionalTest|FinishTest "Default" "YYAYA")
    (else
      (Development|PrintString "NO"))))

(fn ConstructionScript)